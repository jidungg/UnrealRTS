(event `self.ReceiveBeginPlay`
  (if (`self.IsLocalPlayerController`)
    (bind _asbp_game_instance (cast `/Game/Blueprints/Core/BP_GameInstance` (`GameplayStatics.GetGameInstance`)))
    (`/Game/Blueprints/Core/BP_GameInstance.CreateGameMainUI` _asbp_game_instance)))

(event `self.OnBuildButton`
  (`self.Turn On Build Mode`))

(event `self.OnBuildBackButton`
  (`self.TurnOffBuildMode`))

(fn `Turn On Build Mode`
  (`self.SetPlacementMode` true)
  (bind _asbp_game_instance (cast `/Game/Blueprints/Core/BP_GameInstance` (`GameplayStatics.GetGameInstance`)))
  (`/Game/Blueprints/Core/BP_GameInstance.AddUI` _asbp_game_instance "/Game/Blueprints/UI/Common/ActivatableWidget/CAW_BuildMenu.CAW_BuildMenu_C"))

(fn `TurnOffBuildMode`
  (`self.SetPlacementMode` false)
  (bind _asbp_game_instance (cast `/Game/Blueprints/Core/BP_GameInstance` (`GameplayStatics.GetGameInstance`)))
  (`/Game/Blueprints/Core/BP_GameInstance.RemoveUI` _asbp_game_instance))

(fn `UserConstructionScript`)