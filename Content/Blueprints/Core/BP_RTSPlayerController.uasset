(event `self.ReceiveBeginPlay`
  (if (`self.IsLocalPlayerController`)
    (bind _asbp_mobagame_instance (cast `/Game/Blueprints/Core/BP_MOBAGameInstance` (`GameplayStatics.GetGameInstance`)))
    (`/Game/Blueprints/Core/BP_MOBAGameInstance.CreateGameMainUI` _asbp_mobagame_instance)
    (`/Game/Blueprints/Core/BP_MOBAGameInstance.AddUI` _asbp_mobagame_instance "/Game/Blueprints/UI/Common/ActivatableWidget/CAW_GameLayer.CAW_GameLayer_C")))

(event `self.OnBuildButton`
  (`self.TurnOnBuildMode`))

(event `self.OnBuildBackButton`
  (`self.TurnOffBuildMode`))

(fn `TurnOffBuildMode`
  (bind _asbp_mobagame_instance (cast `/Game/Blueprints/Core/BP_MOBAGameInstance` (`GameplayStatics.GetGameInstance`)))
  (`/Game/Blueprints/Core/BP_MOBAGameInstance.RemoveUI` _asbp_mobagame_instance)
  (bind _asrtsplayer_controller (cast `RTSPlayerController` (`GameplayStatics.GetPlayerController` 0)))
  (`self.SetPlacementMode` _asrtsplayer_controller false))

(fn `TurnOnBuildMode`
  (bind _asbp_mobagame_instance (cast `/Game/Blueprints/Core/BP_MOBAGameInstance` (`GameplayStatics.GetGameInstance`)))
  (`/Game/Blueprints/Core/BP_MOBAGameInstance.AddUI` _asbp_mobagame_instance "/Game/Blueprints/UI/Common/ActivatableWidget/CAW_BuildMenu.CAW_BuildMenu_C")
  (`self.SetPlacementMode` true))

(fn `UserConstructionScript`)